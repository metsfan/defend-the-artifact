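; Defendable artifact structure that players claim and then access to trade and unlock skills.
; Its multi-use menu offers Claim or Access; claiming multicasts the claimed state and awards Artifact skill-tree points.
; Accessing opens the artifact UI client-side, filling hexagon trade items and linking the skill tree menu to this actor.
; Skill unlocks go through a server request followed by an immediate UI refresh, while UpdateLevel sets health from a per-level table.
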(event `ClaimArtifact_Multicast`
  (`|ExecutionSequence`
    (:`then_0`
      (set `self.Claimed` true false))
    (:`then_1`
      (`self.OnArtifactClaimed`))))

(event `self.BPClientDoMultiUse`
  (params (ForPC :type "PlayerController Object Reference") (ClientUseIndex :type Integer) (ClientUseName :type Name))
  (if (and (== ClientUseIndex 6001) (`KismetSystemLibrary.IsClient` null))
    (bind _asshooter_player_controller (cast `ShooterPlayerController` ForPC))
    (`|ExecutionSequence`
      (:`then_0`
        (bind _asshooter_hud (cast `ShooterHUD` (`PlayerController.GetHUD` _asshooter_player_controller)))
        (bind _returnvalue (`ShooterHUD.BPShowUIScene` _asshooter_hud "/DefendTheArtifact/UI/ArtifactUI.ArtifactUI_C" null null 0 0))
        (bind _asartifact_ui (cast `/DefendTheArtifact/UI/ArtifactUI` _returnvalue :!pure true))
        (`UI_HexagonConversion.PopulateAvailableTradeItems` (`/DefendTheArtifact/UI/ArtifactUI.Hexagon_Trade_UI` _asartifact_ui) (`|MakeArray` true))
        (set `self.CurrentUI` _asartifact_ui)
        (set `/DefendTheArtifact/UI/Artifact_UI_SkillTreeMenu.ArtifactActor` self (`/DefendTheArtifact/UI/ArtifactUI.Artifact_UI_SkillTreeMenu` _asartifact_ui))))))

(event `ShowArtifactUI`
  (`KismetSystemLibrary.PrintString` null "Show Artifact UI"))

(event `TryUnlockSkill`
  (params (PC :type "ShooterPlayerController Object Reference") (Skill :type Name) (SkillTreeProvider :type "Object Object Reference"))
  (`|ExecutionSequence`
    (:`then_0`
      (`ShooterPlayerController.ServerRequestUnlockSkill` PC Skill SkillTreeProvider))
    (:`then_1`
      (`self.SkillUnlockComplete` Skill))))

(event `SkillUnlockComplete`
  (params (SkillName :type Name))
  (bind _currentui (`self.CurrentUI`))
  (`/Engine/EditorBlueprintResources/StandardMacros.IsValid` _currentui
    (:`Is Valid`
      (`/DefendTheArtifact/UI/Artifact_UI_SkillTreeMenu.RefreshUI` (`/DefendTheArtifact/UI/ArtifactUI.Artifact_UI_SkillTreeMenu` _currentui)))))

(fn `BPGetMultiUseEntries`
  (params (ForPC :type "PlayerController Object Reference") (MultiUseEntries :type "Array of MultiUseEntry Structure (by ref)"))
  (returns (ReturnValue :type "Array of MultiUseEntry Structure"))
  (return (select `bool` (`self.Claimed`) :`false` (`|MakeArray` (make `MultiUseEntry` null "Claim Artifact" 6000)) :`true` (`|MakeArray` (make `MultiUseEntry` null "Access Artifact" 6001)))))

(fn `BPTryMultiUse`
  (params (ForPC :type "PlayerController Object Reference") (UseIndex :type Integer) (UseName :type Name))
  (returns (ReturnValue :type Boolean))
  (`|ExecutionSequence`
    (:`then_0`
      (if (== UseIndex 6000)
        (`self.ClaimArtifact_Multicast`)
        (bind _asshooter_player_state (cast `ShooterPlayerState` (`Controller.PlayerState` ForPC)))
        (`ShooterPlayerState.AddTreeSkillPoints` _asshooter_player_state "Artifact" 50)))
    (:`then_1`
      (return true))))

(fn `UpdateLevel`
  (params (NewLevel :type Integer))
  (`|ExecutionSequence`
    (:`then_0`
      (set `self.Health` (`|GetArrayItem` (`self.HealthLevels`) NewLevel)))))

(fn `UserConstructionScript`)