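; Server-side controller for a Defend the Artifact mode, where an artifact structure faces a dino horde mission.
; BeginPlay finds or spawns the artifact using per-map data.
; InitializeArtifact places floors and spawn points from that data, binds artifact destruction to mission failure, and starts the horde mission with saved state.
; Tick re-snapshots mission state every frame; prevention-zone and ground-trace spawn helpers exist but are unused here.
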(event `self.ReceiveBeginPlay`
  (`|ExecutionSequence`
    (:`then_1`
      (if (`self.HasAuthority`)
        (`|ExecutionSequence`
          (:`then_0`
            (`self.FindOrSpawnArtifact`)))))))

(event `self.ReceiveTick`
  (params (DeltaSeconds :type "Float (single-precision)"))
  (bind _activemission (`self.ActiveMission`))
  (`parent.ReceiveTick` DeltaSeconds)
  (`/Engine/EditorBlueprintResources/ActorMacros.Switch Has Authority`
    (:`Authority`
      (`|ExecutionSequence`
        (:`then_0`
          (`/Engine/EditorBlueprintResources/StandardMacros.IsValid` _activemission
            (:`Is Valid`
              (bind _outstate (`/DefendTheArtifact/Mission/MissionType_ArtifactDinoHorde_Base.CreateMissionState` _activemission))
              (set `self.MissionSaveState` _outstate))))))))

(event `InitializeArtifact`
  (`|ExecutionSequence`
    (:`then_0`
      (`self.SetupSpawnPointsV2`))
    (:`then_1`
      (add `self.OnDestroyed` (`self.ArtifactActor`) (delegate `OnArtifactDestroyed`)))
    (:`then_2`
      (`self.SpawnDinoHordeMission`))))

(event `OnArtifactDestroyed` :!signature `self.OnDestroyed`
  (params (DestroyedActor :type "Actor Object Reference"))
  (bind _activemission (`self.ActiveMission`))
  (`/Engine/EditorBlueprintResources/StandardMacros.IsValid` _activemission
    (:`Is Valid`
      (`/DefendTheArtifact/Mission/MissionType_ArtifactDinoHorde_Base.HandleArtifactDeathFailure` _activemission))))

(fn `FindGroundForPoint`
  (params (Point :type "Vector Structure"))
  (returns (GroundPoint :type "Vector Structure"))
  (bind (_outhit _returnvalue) (`KismetSystemLibrary.LineTraceSingleByProfile` null (- Point (0.0 0.0 20000.0)) (+ Point (0.0 0.0 20000.0)) "GroundTerrain"))
  (return (+ (`KismetMathLibrary.SelectVector` (`.Location` (`GameplayStatics.BreakHitResult` _outhit)) Point _returnvalue) (0.0 0.0 500.0))))

(fn `FindOrSpawnArtifact`
  (bind _outactors (`GameplayStatics.GetAllActorsOfClass` null "/DefendTheArtifact/Actor/BP_DefendArtifactStructure.BP_DefendArtifactStructure_C"))
  (bind _asbp_defend_artifact_structure (cast `/DefendTheArtifact/Actor/BP_DefendArtifactStructure` (`|GetArrayItem` _outactors))
    (:`then`
      (set `self.ArtifactActor` _asbp_defend_artifact_structure))
    (:`CastFailed`
      (`self.SpawnArtifact`))))

(fn `GetArtifactLocationForMap`
  (returns (Location :type "Vector Structure"))
  (bind _returnvalue (`VictoryCore.BPGetPrimaryMapName` null))
  (return (`.ArtifactLocation_3_FEE6E517476EA140F8DE749FC2EE0949` (break `/DefendTheArtifact/Data/MapArtifactData` (`BlueprintMapLibrary.Map_Find` (`self.MapArtifactData`) _returnvalue)))))

(fn `SetupSpawnPoints`
  (bind _spawnpoints (`self.SpawnPoints`))
  (bind _returnvalue (* (`self.StructurePreventionRadius`) 1.25))
  (`|ExecutionSequence`
    (:`then_0`
      (for _array_element (`self.StructurePreventionZones`)
        (`|ExecutionSequence`
          (:`then_0`
            (bind _returnvalue_2 (`self.K2_GetActorLocation` _array_element))
            (`KismetArrayLibrary.Array_Add` _spawnpoints (`self.FindGroundForPoint` _returnvalue_2)))
          (:`then_1`
            (if (> (.x (`self.GetActorScale3D` _array_element)) (.y (`self.GetActorScale3D` _array_element)))
              (`KismetArrayLibrary.Array_Add` _spawnpoints (`self.FindGroundForPoint` (+ _returnvalue_2 (`KismetMathLibrary.MakeVector` _returnvalue))))
              (`KismetArrayLibrary.Array_Add` _spawnpoints (`self.FindGroundForPoint` (- _returnvalue_2 (`KismetMathLibrary.MakeVector` _returnvalue))))
              (else
                (`KismetArrayLibrary.Array_Add` _spawnpoints (`self.FindGroundForPoint` (+ _returnvalue_2 (`KismetMathLibrary.MakeVector` 0.0 _returnvalue))))
                (`KismetArrayLibrary.Array_Add` _spawnpoints (`self.FindGroundForPoint` (- _returnvalue_2 (`KismetMathLibrary.MakeVector` 0.0 _returnvalue))))))))))))

(fn `SetupSpawnPointsV2`
  (bind _returnvalue (`VictoryCore.BPGetPrimaryMapName` null))
  (for _array_element (`.SpawnPoints_6_509EAA284432EB5D4B58588448EDA17B` (break `/DefendTheArtifact/Data/MapArtifactData` (`BlueprintMapLibrary.Map_Find` (`self.MapArtifactData`) _returnvalue)))
    (bind _returnvalue_2 (+ _array_element (0.0 0.0 500.0)))
    (`|SpawnActorFromClass` "/DefendTheArtifact/Actor/SpawnPointFloor.SpawnPointFloor_C" (`KismetMathLibrary.MakeTransform` _returnvalue_2) "AlwaysSpawn" "MultiplyWithRoot" null null)
    (`KismetArrayLibrary.Array_Add` (`self.SpawnPoints`) _returnvalue_2)))

(fn `SpawnArtifact`
  (bind _returnvalue (`|SpawnActorFromClass` "/DefendTheArtifact/Actor/BP_DefendArtifactStructure.BP_DefendArtifactStructure_C" (`KismetMathLibrary.MakeTransform` (`self.GetArtifactLocationForMap`)) "Undefined" "MultiplyWithRoot" null null))
  (set `self.ArtifactActor` _returnvalue)
  (set `self.ArtifactEverSpawned` true))

(fn `SpawnDinoHordeMission`
  (`|ExecutionSequence`
    (:`then_1`
      (bind (_failurereason _returnvalue) (`MissionType.SpawnMission` (cast `ShooterGameState` (`GameplayStatics.GetGameState` (`self.K2_GetWorld`)) :!pure true) "/DefendTheArtifact/Mission/MissionType_ArtifactDinoHorde_Base.MissionType_ArtifactDinoHorde_Base_C" null (`KismetMathLibrary.MakeVector` 0.0) null true))
      (if (> (`KismetStringLibrary.Len` _failurereason) 0)
        (`KismetSystemLibrary.PrintString` null _failurereason)
        (else
          (bind _asmission_type_artifact_dino_horde_base (cast `/DefendTheArtifact/Mission/MissionType_ArtifactDinoHorde_Base` _returnvalue))
          (`/DefendTheArtifact/Mission/MissionType_ArtifactDinoHorde_Base.SetMissionData` _asmission_type_artifact_dino_horde_base (`self.SpawnPoints`) (`self.DinoScript`) (`self.MissionSaveState`) (`self.ArtifactActor`))
          (set `self.ActiveMission` _asmission_type_artifact_dino_horde_base))))))

(fn `SpawnStructurePreventionZones`
  (bind _structurepreventionradius (`self.StructurePreventionRadius`))
  (bind _structurepreventionzones (`self.StructurePreventionZones`))
  (bind (_returnvalue_x _returnvalue_y _returnvalue_z) (`KismetMathLibrary.BreakVector` (`self.K2_GetActorLocation` (`self.ArtifactActor`))))
  (bind _returnvalue (* _structurepreventionradius 5.0))
  (bind _returnvalue_2 (+ (`self.BuildRadius`) (* (`self.StructurePreventionRadius`) 0.5)))
  (`|ExecutionSequence`
    (:`then_0`
      (bind _returnvalue_3 (`|SpawnActorFromClass` "/DefendTheArtifact/Actor/BP_DynamicStructurePreventionZone.BP_DynamicStructurePreventionZone_C" (`KismetMathLibrary.MakeTransform` (`KismetMathLibrary.MakeVector` (+ _returnvalue_x _returnvalue_2) _returnvalue_y _returnvalue_z)) "AlwaysSpawn" "MultiplyWithRoot" null null))
      (`/DefendTheArtifact/Actor/BP_DynamicStructurePreventionZone.UpdateBoxSize` _returnvalue_3 _structurepreventionradius _returnvalue)
      (`KismetArrayLibrary.Array_Add` _structurepreventionzones _returnvalue_3))
    (:`then_1`
      (bind _returnvalue_4 (`|SpawnActorFromClass` "/DefendTheArtifact/Actor/BP_DynamicStructurePreventionZone.BP_DynamicStructurePreventionZone_C" (`KismetMathLibrary.MakeTransform` (`KismetMathLibrary.MakeVector` (- _returnvalue_x _returnvalue_2) _returnvalue_y _returnvalue_z)) "AlwaysSpawn" "MultiplyWithRoot" null null))
      (`/DefendTheArtifact/Actor/BP_DynamicStructurePreventionZone.UpdateBoxSize` _returnvalue_4 _structurepreventionradius _returnvalue)
      (`KismetArrayLibrary.Array_Add` _structurepreventionzones _returnvalue_4))
    (:`then_2`
      (bind _returnvalue_5 (`|SpawnActorFromClass` "/DefendTheArtifact/Actor/BP_DynamicStructurePreventionZone.BP_DynamicStructurePreventionZone_C" (`KismetMathLibrary.MakeTransform` (`KismetMathLibrary.MakeVector` _returnvalue_x (+ _returnvalue_y _returnvalue_2) _returnvalue_z)) "AlwaysSpawn" "MultiplyWithRoot" null null))
      (`/DefendTheArtifact/Actor/BP_DynamicStructurePreventionZone.UpdateBoxSize` _returnvalue_5 _returnvalue _structurepreventionradius)
      (`KismetArrayLibrary.Array_Add` _structurepreventionzones _returnvalue_5))
    (:`then_3`
      (bind _returnvalue_6 (`|SpawnActorFromClass` "/DefendTheArtifact/Actor/BP_DynamicStructurePreventionZone.BP_DynamicStructurePreventionZone_C" (`KismetMathLibrary.MakeTransform` (`KismetMathLibrary.MakeVector` _returnvalue_x (- _returnvalue_y _returnvalue_2) _returnvalue_z)) "AlwaysSpawn" "MultiplyWithRoot" null null))
      (`/DefendTheArtifact/Actor/BP_DynamicStructurePreventionZone.UpdateBoxSize` _returnvalue_6 _returnvalue _structurepreventionradius)
      (`KismetArrayLibrary.Array_Add` _structurepreventionzones _returnvalue_6))))

(fn `UserConstructionScript`
  (`parent.UserConstructionScript`))