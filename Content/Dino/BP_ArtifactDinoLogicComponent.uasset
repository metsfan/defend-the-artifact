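; Logic component for dinos in the artifact defense event that makes them attack the artifact structure.
; On begin play it finds the first BP_DefendArtifactStructure and gives it a very high aggro value on the owning dino AI controller, notifying neighbors.
; Each tick, if the controller has no valid target, it sets the artifact as the target again.
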(event `self.ReceiveBeginPlay`
  (bind _asdino_aicontroller_bp (cast `/Game/PrimalEarth/CoreAI/Dino_AIController_BP` (`self.GetOwner`) :!pure true))
  (bind _outactors (`GameplayStatics.GetAllActorsOfClass` null "/DefendTheArtifact/Actor/BP_DefendArtifactStructure.BP_DefendArtifactStructure_C"))
  (bind _output_get (set `self.Artifact` (`|GetArrayItem` _outactors)))
  (`PrimalDinoAIController.AddToAggro` _asdino_aicontroller_bp _output_get 1000.0 true false false false)
  (`PrimalDinoAIController.UpdateAggro` _asdino_aicontroller_bp))

(event `self.ReceiveTick`
  (params (DeltaSeconds :type "Float (single-precision)"))
  (bind _asdino_aicontroller_bp (cast `/Game/PrimalEarth/CoreAI/Dino_AIController_BP` (`self.GetOwner`) :!pure true))
  (`|ExecutionSequence`
    (:`then_0`
      (bind _returnvalue (`PrimalDinoAIController.GetTarget` _asdino_aicontroller_bp))
      (`/Engine/EditorBlueprintResources/StandardMacros.IsValid` _returnvalue
        (:`Is Not Valid`
          (`PrimalDinoAIController.SetTarget` _asdino_aicontroller_bp (`self.Artifact`) false false))))))